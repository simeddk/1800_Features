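; BP_NPC is an NPC Blueprint that drives a motion smear effect on its mesh from its own velocity.
; BeginPlay creates a dynamic instance of a smear material, assigns it to the first two mesh material slots and starts with no smear.
; Each Tick sets the smear direction opposite to the normalized velocity and scales its amount linearly with speed.
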(event `self.ReceiveBeginPlay`
  (bind _mesh (`self.Mesh`))
  (bind _returnvalue (`KismetMaterialLibrary.CreateDynamicMaterialInstance` "/Game/Materials/Surface/MAT_Smear_Inst1.MAT_Smear_Inst1"))
  (bind _output_get (set `self.Dynamic` _returnvalue))
  (`PrimitiveComponent.SetMaterial` _mesh 0 _output_get)
  (`PrimitiveComponent.SetMaterial` _mesh 1 _output_get)
  (`MaterialInstanceDynamic.SetScalarParameterValue` (`self.Dynamic`) "Amount" 0.0))

(event `self.ReceiveTick`
  (params (DeltaSeconds :type "Float (single-precision)"))
  (bind _returnvalue (`self.GetVelocity`))
  (bind _dynamic (`self.Dynamic`))
  (`MaterialInstanceDynamic.SetVectorParameterValue` _dynamic "Direction" (`KismetMathLibrary.Conv_VectorToLinearColor` (* (`KismetMathLibrary.Normal` _returnvalue) -1.0)))
  (`MaterialInstanceDynamic.SetScalarParameterValue` _dynamic "Amount" (* (`KismetMathLibrary.VSize` _returnvalue) 0.15)))

(fn `UserConstructionScript`)